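; BP_Mortarion is a creature Blueprint under the Pokemon folder that feeds its stats to the enemy side of the combat UI.
; It extends a parent class, overriding ActualiseUI to call the parent, then set the enemy panel's HP bar, level and name through the Player's UICombat widget.
; StartUI and the construction script only defer to the parent, and BeginPlay is disabled.
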(event EventBeginPlay
  (|CallParentFunction) ; This node is disabled and will not be called.\nDrag off pins to build functionality.
)

(event EventStartUI
  (|CallParentFunction))

(event EventActualiseUI
  (params (New%20HP :type Float%20%28double-precision%29) (Max%20HP :type Float%20%28double-precision%29) (Level :type Integer) (Name :type Text))
  (bind _player (Variables|Default|GetPlayer))
  (bind _ui_combat (Variables|/Game/Player/Combat/BP_CombatPlayer.BP_CombatPlayer_C|GetUI_Combat _player))
  (bind _wp_combat_enemy_stats (Variables|/Game/UI/WBP/WBP_Combat_UI_Player.WBP_Combat_UI_Player_C|GetWP_Combat_Enemy_Stats _ui_combat))
  (|CallParentFunction New%20HP Max%20HP Level Name)
  (Progress|SetPercent (Variables|/Game/UI/WBP/WP_Combat_PlayerStat.WP_Combat_PlayerStat_C|GetHP_Bar _wp_combat_enemy_stats) (Math|Float|NormalizetoRange New%20HP 0.0 Max%20HP))
  (Rendering|Components|TextRender|SetText (Variables|/Game/UI/WBP/WP_Combat_PlayerStat.WP_Combat_PlayerStat_C|GetLvl_Text _wp_combat_enemy_stats) (Utilities|Text|ToText(Integer) Level))
  (Rendering|Components|TextRender|SetText (Variables|/Game/UI/WBP/WP_Combat_PlayerStat.WP_Combat_PlayerStat_C|GetName_Text _wp_combat_enemy_stats) Name))

(fn ConstructionScript
  (|CallParentFunction))