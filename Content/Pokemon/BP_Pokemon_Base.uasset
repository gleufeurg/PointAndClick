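; BP_Pokemon_Base is the base Blueprint for a combat Pokémon, holding its HP, level and name.
; One tick after BeginPlay it loads its stats from DT_Pokemon by row name, caches BP_CombatPlayer and starts its UI.
; TakeDamage subtracts HP, refreshes the UI and calls Die at zero or below.
; The UI and death events are empty hooks here, apparently for child Blueprints to implement.
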(event Custom|Start_UI)

(event Custom|Actualise_UI
  (params (New%20HP :type Float%20%28double-precision%29) (Max%20HP :type Float%20%28double-precision%29) (Level :type Integer) (Name :type Text)))

(event Custom|Die)

(event EventTakeDamage
  (params (Damage :type Float%20%28double-precision%29))
  (bind _output_get (Variables|Data|Setcurrent%20HP (- (Variables|Data|Getcurrent%20HP) Damage)))
  (CallFunction|ActualiseUI _output_get (Variables|Data|GetMax%20HP) (Variables|Data|GetLvl) (Variables|Data|GetName))
  (if (<= (Variables|Data|Getcurrent%20HP) 0.0)
    (CallFunction|Die)))

(event EventBeginPlay
  (bind _data (Variables|Data|GetData))
  (Utilities|FlowControl|DelayUntilNextTick)
  (bind _returnvalue (Utilities|GetDataTableRow "/Game/Pokemon/DT_Pokemon.DT_Pokemon" (.rowname _data))
    (:then
      (bind _output_get (Variables|Data|SetMax%20HP (.HP (Utilities|Struct|BreakF_Pokemon _returnvalue))))
      (Variables|Data|Setcurrent%20HP _output_get)
      (Variables|Data|SetLvl (.lvl (Utilities|Struct|BreakF_Pokemon _returnvalue)))
      (Variables|Data|SetName (Utilities|Text|ToText(Name) (.rowname _data)))
      (bind _returnvalue_2 (Actor|GetActorOfClass "/Game/Player/Combat/BP_CombatPlayer.BP_CombatPlayer_C"))
      (Variables|Default|SetPlayer _returnvalue_2)
      (CallFunction|StartUI))))

(fn ConstructionScript)