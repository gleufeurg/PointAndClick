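; BP_Jaghatai is the player-side combat Pokémon Jaghatai, a child Blueprint that extends shared parent behavior.
; On BeginPlay it adds a StormVoice component as Attack1, finds BP_CombatPlayer and registers itself as that player's CurrentPokemon.
; ActualiseUI calls the parent, then writes normalized HP, level and name to the player's stat widget in the combat UI.
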(event EventBeginPlay
  (|CallParentFunction)
  (bind _returnvalue (AddComponent|AddBPCStormVoice))
  (Variables|Default|SetAttack_1 _returnvalue)
  (bind _returnvalue_2 (Actor|GetActorOfClass "/Game/Player/Combat/BP_CombatPlayer.BP_CombatPlayer_C"))
  (bind _output_get (Variables|Default|SetPlayer _returnvalue_2))
  (Variables|/Game/Player/Combat/BP_CombatPlayer.BP_CombatPlayer_C|SetCurrent%20Pokemon _output_get self))

(event EventStartUI
  (|CallParentFunction))

(event EventActualiseUI
  (params (New%20HP :type Float%20%28double-precision%29) (Max%20HP :type Float%20%28double-precision%29) (Level :type Integer) (Name :type Text))
  (bind _player (Variables|Default|GetPlayer))
  (bind _ui_combat (Variables|/Game/Player/Combat/BP_CombatPlayer.BP_CombatPlayer_C|GetUI_Combat _player))
  (bind _wp_combat_playerstat (Variables|/Game/UI/WBP/WBP_Combat_UI_Player.WBP_Combat_UI_Player_C|GetWP_Combat_PlayerStat _ui_combat))
  (|CallParentFunction New%20HP Max%20HP Level Name)
  (Progress|SetPercent (Variables|/Game/UI/WBP/WP_Combat_PlayerStat.WP_Combat_PlayerStat_C|GetHP_Bar _wp_combat_playerstat) (Math|Float|NormalizetoRange New%20HP 0.0 Max%20HP))
  (Rendering|Components|TextRender|SetText (Variables|/Game/UI/WBP/WP_Combat_PlayerStat.WP_Combat_PlayerStat_C|GetLvl_Text _wp_combat_playerstat) (Utilities|Text|ToText(Integer) Level))
  (Rendering|Components|TextRender|SetText (Variables|/Game/UI/WBP/WP_Combat_PlayerStat.WP_Combat_PlayerStat_C|GetName_Text _wp_combat_playerstat) Name))

(fn ConstructionScript
  (|CallParentFunction))